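; A time portal actor whose projector mirrors the player's view relative to a teleport destination.
; Each tick, PortalProjector takes the player camera's world rotation, with yaw offset by the difference between TeleportLocation and PortalTrigger.
; AllowThroughTrigger clears IsActive when a ChronoCharacter enters and restores it half a second after exit.
; The graph contains no teleport logic and does not read IsActive.
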(event `self.ReceiveTick`
  (params (DeltaSeconds :type "Float (single-precision)"))
  (bind (_returnvalue_roll _returnvalue_pitch _returnvalue_yaw) (`KismetMathLibrary.BreakRotator` (`SceneComponent.K2_GetComponentRotation` (`self.PortalTrigger`))))
  (bind (_returnvalue_roll_2 _returnvalue_pitch_2 _returnvalue_yaw_2) (`KismetMathLibrary.BreakRotator` (`SceneComponent.K2_GetComponentRotation` (`self.TeleportLocation`))))
  (bind (_returnvalue_roll_3 _returnvalue_pitch_3 _returnvalue_yaw_3) (`KismetMathLibrary.BreakRotator` (`SceneComponent.K2_GetComponentRotation` (`PlayerCameraManager.TransformComponent` (`PlayerController.PlayerCameraManager` (`GameplayStatics.GetPlayerController` 0))))))
  ;[1 0 0.6797] Comment
  (`SceneComponent.K2_SetWorldRotation` (`self.PortalProjector`) (`KismetMathLibrary.MakeRotator` _returnvalue_roll_3 _returnvalue_pitch_3 (+ _returnvalue_yaw_3 (- _returnvalue_yaw_2 _returnvalue_yaw))) false false))

(event `self.AllowThroughTrigger.OnComponentBeginOverlap`
  (params (OverlappedComponent :type "PrimitiveComponent Object Reference") (OtherActor :type "Actor Object Reference") (OtherComp :type "PrimitiveComponent Object Reference") (OtherBodyIndex :type Integer) (bFromSweep :type Boolean) (SweepResult :type "HitResult Structure (by ref)"))
  (cast `ChronoCharacter` OtherActor)
  (set `self.bIsActive` false))

(event `self.AllowThroughTrigger.OnComponentEndOverlap`
  (params (OverlappedComponent :type "PrimitiveComponent Object Reference") (OtherActor :type "Actor Object Reference") (OtherComp :type "PrimitiveComponent Object Reference") (OtherBodyIndex :type Integer))
  (cast `ChronoCharacter` OtherActor)
  (`KismetSystemLibrary.Delay` 0.5)
  (set `self.bIsActive` true))

(fn `UserConstructionScript`)