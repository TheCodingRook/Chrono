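; BP_BatteryMedium is a medium battery pickup that shows an electric arc to the player who hits it.
; The first hit on PickupMesh sets a one-shot flag, even if the actor is not BP_Player.
; For a player, it attaches a beam emitter and re-aims it at the WeaponSocket in an endless short-delay loop.
; BatteryPower is unused, so no power is granted here.
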(event `self.PickupMesh.OnComponentHit`
  (params (HitComponent :type "PrimitiveComponent Object Reference") (OtherActor :type "Actor Object Reference") (OtherComp :type "PrimitiveComponent Object Reference") (NormalImpulse :type "Vector Structure") (Hit :type "HitResult Structure (by ref)"))
  (if (not (`self.FirstHit`))
    (set `self.FirstHit` true)
    (bind _asbp_player (cast `/Game/Player/Blueprints/BP_Player` OtherActor))
    (bind _returnvalue (`GameplayStatics.SpawnEmitterAttached` "/Game/Projectiles/Effects/ParticleSystems/P_electricity_arc.P_electricity_arc" (`self.PickupMesh`)))
    (`ParticleSystemComponent.SetBeamTargetPoint` _returnvalue 0 (`SceneComponent.GetSocketLocation` (`Character.Mesh` _asbp_player) "WeaponSocket") 0 :!label _label)
    (`KismetSystemLibrary.Delay` 0.1)
    (goto _label)))

(fn `UserConstructionScript`)