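; Puzzle-driven wooden half-panel door that swings open when all its linked puzzle elements are active and closes when one is untriggered.
; On BeginPlay it gathers PuzzleElement components from the Puzzle's actor list and binds to their trigger events, warning if none exist.
; A DoorRotation timeline adds incremental yaw, signed by open/close direction and FlipRotation, while accumulated rotation stays below MaximumOffset.
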(event `self.ReceiveBeginPlay`
  (bind _puzzle (`self.Puzzle`))
  (bind _returnvalue (`PuzzleComponent.GetPuzzleElementsList` _puzzle))
  (for _array_element (`PuzzleComponent.GetActorsList` _puzzle)
    (bind _returnvalue_2 (`self.GetComponentByClass` _array_element "/Script/Chrono.PuzzleElement"))
    (`/Engine/EditorBlueprintResources/StandardMacros.IsValid` _returnvalue_2
      (:`Is Valid`
        (`PuzzleComponent.AddToElementsList` (`self.Puzzle`) _returnvalue_2))))
  (if (`KismetArrayLibrary.Array_IsValidIndex` _returnvalue)
    (for _array_element_2 _returnvalue
      (add `PuzzleElement.OnPuzzleElementTriggered` _array_element_2 (delegate `OnElementTriggered_Event`))
      (add `PuzzleElement.OnPuzzleElementUnTriggered` _array_element_2 (delegate `OnElementUnTriggered_Event`)))
    (else
      (`KismetSystemLibrary.PrintString` "WARNING! No Puzzle Elements found for this object."))))

(event `OnElementTriggered_Event`
  (`self.Attempt Door Open`))

(event `OnElementUnTriggered_Event`
  (`self.Close Door`))

(event `Attempt Door Open`
  (bind (_returnvalue_roll _returnvalue_pitch _returnvalue_yaw) (`KismetMathLibrary.BreakRotator` (`SceneComponent.K2_GetComponentRotation` (`self.StaticMeshComponent`))))
  (if (`PuzzleComponent.AreAllPuzzleElementsActive` (`self.Puzzle`))
    (`|ExecutionSequence`
      (:`then_0`
        (set `self.Rotation Toggle` 1.0))
      (:`then_1`
        (set `self.Cumulative Offset` 0.0)
        (bind (_direction _degreerotation) (`Timeline|DoorRotation` :!label _label)
          (:`Update`
            (bind _output_get (set `self.Cumulative Offset` (`KismetMathLibrary.FClamp` (+ (`self.Cumulative Offset`) (`KismetMathLibrary.Abs` _degreerotation)) 0.0 (`self.Maximum Offset`))))
            (if (< _output_get (`self.Maximum Offset`))
              (`self.K2_SetActorRotation` (`KismetMathLibrary.MakeRotator` _returnvalue_roll _returnvalue_pitch (+ _returnvalue_yaw (* _degreerotation (select `bool` (`self.Flip rotation`) :`false` 1.0 :`true` -1.0 :!type "Float (single-precision)") (stale `Close Door` _output_get))))))))))))

(event `Close Door`
  (`|ExecutionSequence`
    (:`then_0`
      (set `self.Cumulative Offset` 0.0))
    (:`then_1`
      (bind _output_get (set `self.Rotation Toggle` -1.0))
      (goto _label :!via `Reverse`))))

(fn `UserConstructionScript`)