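; A stone brick puzzle door that moves vertically when all its linked puzzle elements are active.
; On BeginPlay it collects PuzzleElement components from the Puzzle's actor list and binds their triggered and untriggered events, warning if none exist.
; A timeline adds height increments to the actor's location each update, capped by a cumulative maximum offset.
; Any untrigger flips the direction sign and reverses the timeline to close the door.
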(event `self.ReceiveBeginPlay`
  (bind _puzzle (`self.Puzzle`))
  (bind _returnvalue (`PuzzleComponent.GetPuzzleElementsList` _puzzle))
  (for _array_element (`PuzzleComponent.GetActorsList` _puzzle)
    (bind _returnvalue_2 (`self.GetComponentByClass` _array_element "/Script/Chrono.PuzzleElement"))
    (`/Engine/EditorBlueprintResources/StandardMacros.IsValid` _returnvalue_2
      (:`Is Valid`
        (`PuzzleComponent.AddToElementsList` (`self.Puzzle`) _returnvalue_2))))
  (if (`KismetArrayLibrary.Array_IsValidIndex` _returnvalue)
    (for _array_element_2 _returnvalue
      (add `PuzzleElement.OnPuzzleElementTriggered` _array_element_2 (delegate `OnElementTriggered_Event`))
      (add `PuzzleElement.OnPuzzleElementUnTriggered` _array_element_2 (delegate `OnElementUnTriggered_Event`)))
    (else
      (`KismetSystemLibrary.PrintString` "WARNING! No Puzzle Elements found for this object."))))

(event `OnElementTriggered_Event`
  (`self.AttemptDoorOpen`))

(event `OnElementUnTriggered_Event`
  (`self.CloseDoor`))

(event `AttemptDoorOpen`
  (bind (_returnvalue_x _returnvalue_y _returnvalue_z) (`KismetMathLibrary.BreakVector` (`self.K2_GetActorLocation`)))
  ;[1 0.5156 0] Operate this door according to the status of triggers
  (if (`PuzzleComponent.bAreAllPuzzleElementsActive` (`self.Puzzle`))
    (set `self.DoorOffsetToggle` 1.0)
    (set `self.CumulativeOffset` 0.0)
    (bind (_direction _heightadjustment) (`Timeline|DoorHeightTimeline` :!label _label)
      (:`Update`
        (bind _output_get (set `self.CumulativeOffset` (`KismetMathLibrary.FClamp` (+ (`self.CumulativeOffset`) (`KismetMathLibrary.Abs` _heightadjustment)) 0.0 (`self.MaximumOffset`))))
        (if (< _output_get (`self.MaximumOffset`))
          (`self.K2_SetActorLocation` (`KismetMathLibrary.MakeVector` _returnvalue_x _returnvalue_y (+ _returnvalue_z (* _heightadjustment (stale `CloseDoor` _output_get))))))))))

(event `CloseDoor`
  ;[1 0.5156 0] Operate this door according to the status of triggers
  (bind _output_get (set `self.DoorOffsetToggle` -1.0))
  (set `self.CumulativeOffset` 0.0)
  (goto _label :!via `Reverse`))

(fn `UserConstructionScript`)