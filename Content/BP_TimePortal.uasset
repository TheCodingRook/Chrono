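; BP_TimePortal is a wall portal that teleports characters when its TimeWindow is visible.
; A BP_RifleProjectile overlapping the Wall toggles TimeWindow visibility.
; A Character hitting the Wall while the window is visible moves to the second SceneCapture2D actor found in the level, taking its yaw.
; ElevateWall, not called here, sets the actor's location to the world origin.
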(event `self.Wall.OnComponentBeginOverlap`
  (params (OverlappedComponent :type "PrimitiveComponent Object Reference") (OtherActor :type "Actor Object Reference") (OtherComp :type "PrimitiveComponent Object Reference") (OtherBodyIndex :type Integer) (bFromSweep :type Boolean) (SweepResult :type "HitResult Structure (by ref)"))
  (cast `/Game/Projectiles/BP_RifleProjectile` OtherActor)
  (`SceneComponent.ToggleVisibility` (`self.TimeWindow`) false))

(event `self.Wall.OnComponentHit`
  (params (HitComponent :type "PrimitiveComponent Object Reference") (OtherActor :type "Actor Object Reference") (OtherComp :type "PrimitiveComponent Object Reference") (NormalImpulse :type "Vector Structure") (Hit :type "HitResult Structure (by ref)"))
  (bind _ascharacter (cast `Character` OtherActor))
  (if (`SceneComponent.IsVisible` (`self.TimeWindow`))
    (bind _outactors (`GameplayStatics.GetAllActorsOfClass` "/Script/Engine.SceneCapture2D"))
    (bind _output (`|GetArrayItem` _outactors 1))
    (`self.K2_SetActorLocation` _ascharacter (`self.K2_GetActorLocation` _output) false true)
    (`self.K2_SetActorRotation` _ascharacter (`KismetMathLibrary.MakeRotator` 0.0 0.0 (.yaw (`self.K2_GetActorRotation` _output))) false)))

(fn `ElevateWall`
  (`self.K2_SetActorLocation` (0.0 0.0 0.0)))

(fn `UserConstructionScript`)