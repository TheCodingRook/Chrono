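; BP_PushToMakeTrigger is a trigger actor that changes its mesh material while a Character overlaps it, giving visual on/off feedback.
; The construction script caches the mesh's slot 0 material as the original.
; Begin overlap with a Character swaps that slot to the MI_TriggerOn material, and end overlap restores the cached one, without counting multiple overlapping characters.
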(event `self.StaticMeshComponent.OnComponentBeginOverlap`
  (params (OverlappedComponent :type "PrimitiveComponent Object Reference") (OtherActor :type "Actor Object Reference") (OtherComp :type "PrimitiveComponent Object Reference") (OtherBodyIndex :type Integer) (bFromSweep :type Boolean) (SweepResult :type "HitResult Structure (by ref)"))
  (cast `Character` OtherActor)
  (`PrimitiveComponent.SetMaterial` (`self.StaticMeshComponent`) 0 "/Game/Triggers/Materials/MI_TriggerOn.MI_TriggerOn"))

(event `self.StaticMeshComponent.OnComponentEndOverlap`
  (params (OverlappedComponent :type "PrimitiveComponent Object Reference") (OtherActor :type "Actor Object Reference") (OtherComp :type "PrimitiveComponent Object Reference") (OtherBodyIndex :type Integer))
  (cast `Character` OtherActor)
  (`PrimitiveComponent.SetMaterial` (`self.StaticMeshComponent`) 0 (`self.OriginalMaterial`)))

(fn `UserConstructionScript`
  (set `self.OriginalMaterial` (`PrimitiveComponent.GetMaterial` (`self.StaticMeshComponent`) 0)))