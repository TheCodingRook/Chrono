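; BP_Brazier is an interactable brazier trigger that uses BPLightInteraction and can prompt the player to light a torch.
; When it starts unlit, BeginPlay turns both indicator materials off and starts a randomized point-light flicker loop.
; CombustionSphere overlaps show the "(F) - Light Torch" widget for an unlit BP_Torch at a lit brazier, removing it on exit.
; QueryComboProp checks the BP_ChronoCharacter's attached actors for a lit torch.
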(event `self.ReceiveBeginPlay`
  ;[0 1 0.4609] Set light indicators for brazier
  (if (not (`self.IsLit?`))
    (`|ExecutionSequence`
      (:`then_0`
        (`PrimitiveComponent.SetMaterial` (`self.Light Indicator 1`) 0 "/Game/Triggers/Materials/MI_TriggerOff.MI_TriggerOff"))
      (:`then_1`
        (`PrimitiveComponent.SetMaterial` (`self.Light Indicator 2`) 0 "/Game/Triggers/Materials/MI_TriggerOff.MI_TriggerOff"))
      (:`then_2`
        ;[0.8516 0 1] Flicker
        (`LightComponent.SetIntensity` (`self.PointLight`) (`KismetMathLibrary.RandomFloatInRange` 12.0 20.0) :!label _label)
        (`KismetSystemLibrary.Delay` (`KismetMathLibrary.RandomFloatInRange` 0.0 0.2))
        (goto _label)))))

(event `self.CombustionSphere.OnComponentBeginOverlap`
  (params (OverlappedComponent :type "PrimitiveComponent Object Reference") (OtherActor :type "Actor Object Reference") (OtherComp :type "PrimitiveComponent Object Reference") (OtherBodyIndex :type Integer) (bFromSweep :type Boolean) (SweepResult :type "HitResult Structure (by ref)"))
  (bind _asbp_torch (cast `/Game/Triggers/Blueprints/BP_Torch` OtherActor))
  (if (`/Game/Triggers/Blueprints/BP_Torch.IsLit?` _asbp_torch)
    _
    (elif (`self.IsLit?`)
      (bind _returnvalue (`|CreateWidget` "/Game/UI/InteractionText.InteractionText_C" (`GameplayStatics.GetPlayerController` 0)))
      (bind _output_get (set `self.LightTorchWidget` _returnvalue))
      (set `/Game/UI/InteractionText.InteractionText` "(F) - Light Torch" _output_get)
      (set `/Game/UI/InteractionText.InteractableActor` self _output_get)
      (set `/Game/UI/InteractionText.TextColor` (make `SlateColor` (struct :`R` 1.0 :`G` 1.0 :`B` 1.0 :`A` 1.0)) (`self.LightTorchWidget`))
      (`UserWidget.AddToViewport` (`self.LightTorchWidget`) 0))))

(event `self.CombustionSphere.OnComponentEndOverlap`
  (params (OverlappedComponent :type "PrimitiveComponent Object Reference") (OtherActor :type "Actor Object Reference") (OtherComp :type "PrimitiveComponent Object Reference") (OtherBodyIndex :type Integer))
  (bind _lighttorchwidget (`self.LightTorchWidget`))
  (cast `/Game/Triggers/Blueprints/BP_Torch` OtherActor)
  (`/Engine/EditorBlueprintResources/StandardMacros.IsValid` _lighttorchwidget
    (:`Is Valid`
      (`Widget.RemoveFromParent` _lighttorchwidget))))

(fn `QueryComboProp`
  (params (InPawn :type "Pawn Object Reference"))
  (returns (Availability :type Boolean))
  (locals (`FoundLitTorch?` :type Boolean :default false))
  (bind _asbp_chrono_character (cast `/Game/Player/Blueprints/BP_ChronoCharacter` InPawn))
  (for _array_element (`self.GetAttachedActors` _asbp_chrono_character true)
    ;[1 0.9375 0] If we find a BP_Torch that is lit then return true!
    (bind _asbp_torch (cast `/Game/Triggers/Blueprints/BP_Torch` _array_element))
    (set `local.FoundLitTorch?` (`/Game/Triggers/Blueprints/BP_Torch.IsLit?` _asbp_torch)))
  (return (`local.FoundLitTorch?`)))

(fn `UserConstructionScript`
  (set `self.InteractionCommand` (`self.BP_LightInteraction`)))