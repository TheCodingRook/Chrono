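; Interaction component for a BP_Brazier that handles fire lighting between the brazier and a torch attached to the instigator.
; LightFire searches the instigator's attached actors and proceeds when exactly one of torch and brazier is lit.
; LightUpBrazier shows fire and light, updates indicator materials, flags its puzzle element as triggered and removes the interaction widget.
; LightUpTorch sets the torch's IsLit but hides its fire and light.
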(event `self.LightFire`
  (params (Instigator :type "ChronoCharacter Object Reference"))
  (bind _asbp_brazier (cast `/Game/Triggers/Blueprints/BP_Brazier` (`self.GetOwner`)))
  (for _array_element (`Actor.GetAttachedActors` Instigator true)
    (bind _asbp_torch (cast `/Game/Triggers/Blueprints/BP_Torch` _array_element))
    (if (xor (`/Game/Triggers/Blueprints/BP_Torch.IsLit?` _asbp_torch) (`/Game/Triggers/Blueprints/BP_Brazier.IsLit?` _asbp_brazier))
      (`self.LightUpBrazier` _asbp_brazier)
      (`self.LightUpTorch` _asbp_torch))))

(fn `LightUpBrazier`
  (params (BrazierToLightUp :type "/Game/Triggers/Blueprints/BP_Brazier Object Reference"))
  (`|ExecutionSequence`
    (:`then_0`
      (set `/Game/Props/Blueprints/BP_InteractableProp.IsWidgetNecessary?` false BrazierToLightUp))
    (:`then_1`
      (set `/Game/Triggers/Blueprints/BP_Brazier.IsLit?` true BrazierToLightUp))
    (:`then_2`
      (`SceneComponent.SetVisibility` (`/Game/Triggers/Blueprints/BP_Brazier.Fire` BrazierToLightUp) true false))
    (:`then_3`
      (`SceneComponent.SetVisibility` (`/Game/Triggers/Blueprints/BP_Brazier.PointLight` BrazierToLightUp) true false))
    (:`then_4`
      (`PrimitiveComponent.SetMaterial` (`/Game/Triggers/Blueprints/BP_Brazier.Light Indicator 1` BrazierToLightUp) 0 "/Game/PolygonPrototype/Materials/Mat_PolygonPrototype_01.Mat_PolygonPrototype_01"))
    (:`then_5`
      (`PrimitiveComponent.SetMaterial` (`/Game/Triggers/Blueprints/BP_Brazier.Light Indicator 2` BrazierToLightUp) 0 null))
    (:`then_6`
      (`PuzzleElement.SetElementTriggeredFlag` (`/Game/Triggers/Blueprints/BP_Brazier.PuzzleElement` BrazierToLightUp) true))
    (:`then_7`
      (`Widget.RemoveFromParent` (`/Game/Props/Blueprints/BP_InteractableProp.InteractionWidget` BrazierToLightUp)))))

(fn `LightUpTorch`
  (params (TorchToLightUp :type "/Game/Triggers/Blueprints/BP_Torch Object Reference"))
  (`|ExecutionSequence`
    (:`then_0`
      (set `/Game/Triggers/Blueprints/BP_Torch.IsLit?` true TorchToLightUp))
    (:`then_1`
      (`SceneComponent.SetVisibility` (`/Game/Triggers/Blueprints/BP_Torch.Fire` TorchToLightUp) false false))
    (:`then_2`
      (`SceneComponent.SetVisibility` (`/Game/Triggers/Blueprints/BP_Torch.PointLight` TorchToLightUp) false false))))