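; BP_OnOffTrigger is a trigger actor that visually toggles between off and on states when a Character begins overlapping its static mesh.
; The construction script caches the mesh's slot 0 material as the off look.
; Each overlap flips the Toggled flag and swaps between that original material and MI_TriggerOn.
; It drives no other logic in these graphs.
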(event `self.StaticMeshComponent.OnComponentBeginOverlap`
  (params (OverlappedComponent :type "PrimitiveComponent Object Reference") (OtherActor :type "Actor Object Reference") (OtherComp :type "PrimitiveComponent Object Reference") (OtherBodyIndex :type Integer) (bFromSweep :type Boolean) (SweepResult :type "HitResult Structure (by ref)"))
  (bind _staticmeshcomponent (`self.StaticMeshComponent`))
  (cast `Character` OtherActor)
  (if (`self.Toggled`)
    (`PrimitiveComponent.SetMaterial` _staticmeshcomponent 0 (`self.OriginalMaterial`))
    (set `self.Toggled` false)
    (else
      (`PrimitiveComponent.SetMaterial` _staticmeshcomponent 0 "/Game/Triggers/Materials/MI_TriggerOn.MI_TriggerOn")
      (set `self.Toggled` true))))

(fn `UserConstructionScript`
  (set `self.OriginalMaterial` (`PrimitiveComponent.GetMaterial` (`self.StaticMeshComponent`) 0)))