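; Brick cut-stone pressure plate that acts as a puzzle trigger for sufficiently heavy objects.
; Trigger volume overlaps from components above a mass threshold set or clear the PuzzleElement's triggered flag and fire its triggered or untriggered call.
; A timeline plays or reverses to shift the actor vertically, with a sign toggle choosing direction and an accumulated offset capped at MaximumOffset limiting travel.
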(event `self.TriggerVolume.OnComponentBeginOverlap`
  (params (OverlappedComponent :type "PrimitiveComponent Object Reference") (OtherActor :type "Actor Object Reference") (OtherComp :type "PrimitiveComponent Object Reference") (OtherBodyIndex :type Integer) (bFromSweep :type Boolean) (SweepResult :type "HitResult Structure (by ref)"))
  (bind (_returnvalue_x _returnvalue_y _returnvalue_z) (`KismetMathLibrary.BreakVector` (`self.K2_GetActorLocation`)))
  (bind _puzzleelement (`self.PuzzleElement`))
  (if (>= (`PrimitiveComponent.GetMass` OtherComp) 100.0)
    (`PuzzleElement.SetElementTriggeredFlag` _puzzleelement true)
    (`PuzzleElement.OnPuzzleElementTriggered` _puzzleelement)
    (set `self.TriggerPlateOffsetToggle` 1.0)
    (set `self.CumulativeOffset` 0.0)
    (bind (_direction _heightadjustment) (`Timeline|Timeline_0` :!label _label)
      (:`Update`
        (bind _output_get (set `self.CumulativeOffset` (`KismetMathLibrary.FClamp` (+ (`self.CumulativeOffset`) (`KismetMathLibrary.Abs` _heightadjustment)) 0.0 (`self.MaximumOffset`))))
        (if (< _output_get (`self.MaximumOffset`))
          (`self.K2_SetActorLocation` (`KismetMathLibrary.MakeVector` _returnvalue_x _returnvalue_y (+ _returnvalue_z (* _heightadjustment (stale `self.TriggerVolume.OnComponentEndOverlap` _output_get))))))))))

(event `self.TriggerVolume.OnComponentEndOverlap`
  (params (OverlappedComponent :type "PrimitiveComponent Object Reference") (OtherActor :type "Actor Object Reference") (OtherComp :type "PrimitiveComponent Object Reference") (OtherBodyIndex :type Integer))
  (bind _puzzleelement (`self.PuzzleElement`))
  (if (>= (`PrimitiveComponent.GetMass` OtherComp) 100.0)
    (`PuzzleElement.SetElementTriggeredFlag` _puzzleelement false)
    (`PuzzleElement.OnPuzzleElementUnTriggered` _puzzleelement)
    (bind _output_get (set `self.TriggerPlateOffsetToggle` -1.0))
    (set `self.CumulativeOffset` 0.0)
    (goto _label :!via `Reverse`)))

(fn `UserConstructionScript`)