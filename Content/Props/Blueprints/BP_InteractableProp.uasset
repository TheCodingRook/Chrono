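; BP_InteractableProp is a prop the player can interact with, showing an on-screen prompt when the player's pawn is nearby.
; On overlap it creates an InteractionText widget labeled with grab text and prop name, then registers its interaction command with ChronoGameInstance.
; End overlap removes the widget and deregisters the command.
; GrabbingAbility events on BP_ChronoCharacter toggle the interacted flag, hiding the prompt and blocking new ones during interaction.
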(event `self.ReceiveBeginPlay`
  (bind _asbp_chrono_character (cast `/Game/Player/Blueprints/BP_ChronoCharacter` (`GameplayStatics.GetPlayerCharacter` 0)))
  (bind _grabbingability (`/Game/Player/Blueprints/BP_ChronoCharacter.GrabbingAbility` _asbp_chrono_character))
  (add `GrabbingAbility.OnPropInteraction` _grabbingability (delegate `RemoveWidget`))
  (add `GrabbingAbility.OnEndedPropInteraction` _grabbingability (delegate `ReenableWidget`)))

(event `RemoveWidget`
  (bind _propwidget (`self.PropWidget`))
  ;[0.4531 0 1] Remove UMG if Player interacts with the prop
  (`self.SetIsInteractedWith` true)
  (`/Engine/EditorBlueprintResources/StandardMacros.IsValid` _propwidget
    (:`Is Valid`
      (`Widget.RemoveFromParent` _propwidget))))

(event `ReenableWidget`
  ;[0 0.625 1] Re-enable UMG
  (`self.SetIsInteractedWith` false))

(event `self.ReceiveActorBeginOverlap`
  (params (OtherActor :type "Actor Object Reference"))
  (bind _returnvalue (`GameplayStatics.GetPlayerController` 0))
  (bind _aspawn (cast `Pawn` OtherActor))
  (if (and (== _aspawn (`Controller.K2_GetPawn` _returnvalue)) (not (`self.IsInteractedWith`)))
    ;[0 1 0.7422] Add the action widget for the prop
    (bind _returnvalue_2 (`|CreateWidget` "/Game/UI/InteractionText.InteractionText_C" _returnvalue))
    (set `self.PropWidget` _returnvalue_2)
    (set `/Game/UI/InteractionText.InteractableActor` self _returnvalue_2)
    (set `/Game/UI/InteractionText.InteractionText` (`KismetSystemLibrary.MakeLiteralText` (`KismetTextLibrary.Conv_StringToText` (`KismetStringLibrary.Concat_StrStr` (`KismetTextLibrary.Conv_TextToString` (`self.GrabText`)) " " (`KismetTextLibrary.Conv_TextToString` (`self.GetPropName`))))) _returnvalue_2)
    (`UserWidget.AddToViewport` _returnvalue_2 0)
    ;[1 0.6797 0] Register the specifc action command type with the GameInstance
    (bind _aschrono_game_instance (cast `ChronoGameInstance` (`GameplayStatics.GetGameInstance`)))
    (`ChronoGameInstance.RegisterCurrentInteractionCommand` _aschrono_game_instance (`self.GetInteractionCommand`))))

(event `self.ReceiveActorEndOverlap`
  (params (OtherActor :type "Actor Object Reference"))
  (bind _aspawn (cast `Pawn` OtherActor))
  (if (== _aspawn (`Controller.K2_GetPawn` (`GameplayStatics.GetPlayerController` 0)))
    (`Widget.RemoveFromParent` (`self.PropWidget`))
    (bind _aschrono_game_instance (cast `ChronoGameInstance` (`GameplayStatics.GetGameInstance`)))
    (`ChronoGameInstance.DeRegisterCurrentInteractionCommand` _aschrono_game_instance)))

(fn `UserConstructionScript`)