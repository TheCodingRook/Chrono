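; Interaction component on BP_Chest that unlocks and opens the chest when the instigator carries a BP_ChestKey.
; UnlockProp searches the instigator's attached actors for a key, offsets the lid instantly, flags the chest unlocked and disables both props' widgets.
; DropKey releases the player's grabbed object, then the key snaps to the lock's KeySocket.
; The key's interaction command is popped from ChronoGameInstance in DropKey and again after attachment.
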(event `self.UnlockProp`
  (params (Instigator :type "Actor Object Reference"))
  (bind _chesttounlock (`self.ChestToUnlock`))
  (bind _keytouse (`self.KeyToUse`))
  (bind _lid (`/Game/Props/Blueprints/BP_Chest.Lid` (`self.ChestToUnlock`)))
  (bind _asbp_chest (cast `/Game/Props/Blueprints/BP_Chest` (`self.GetOwner`)))
  (bind _output_get (set `self.ChestToUnlock` _asbp_chest))
  (if (not (`/Game/Props/Blueprints/BP_Chest.IsAlreadyUnlocked?` _output_get))
    (for _array_element (`Actor.GetAttachedActors` Instigator true)
      (bind _asbp_chest_key (cast `/Game/Props/Blueprints/BP_ChestKey` _array_element))
      (set `self.KeyToUse` _asbp_chest_key)
      ;[0 0.1328 1] Open lid
      (`SceneComponent.K2_AddRelativeRotation` _lid (struct :`Pitch` 50.0) false false)
      (`SceneComponent.K2_AddRelativeLocation` _lid (10.0 0.0 28.0) false false)
      (`/Game/Props/Blueprints/BP_Chest.OnOpenLid` (`self.ChestToUnlock`))
      ;[0.4062 0 1] De-activate the Chest unlocking action (inc. widget)
      (`/Game/Props/Blueprints/BP_InteractableProp.RemoveWidget` _chesttounlock)
      (set `/Game/Props/Blueprints/BP_InteractableProp.IsWidgetNecessary?` false _chesttounlock)
      (set `/Game/Props/Blueprints/BP_Chest.IsAlreadyUnlocked?` true (`self.ChestToUnlock`))
      (`self.DropKey`)
      ;[1 0 0.5156] De-activate the Key's grabbing action (inc. widget) and attach it from player to the chest's lid
      (`/Game/Props/Blueprints/BP_InteractableProp.RemoveWidget` _keytouse)
      (set `/Game/Props/Blueprints/BP_InteractableProp.IsWidgetNecessary?` false _keytouse)
      (`Actor.K2_AttachToComponent` (`self.KeyToUse`) (`/Game/Props/Blueprints/BP_Chest.Lock` (`self.ChestToUnlock`)) "KeySocket" "SnapToTarget" "SnapToTarget" "SnapToTarget" true)
      (bind _aschrono_game_instance (cast `ChronoGameInstance` (`GameplayStatics.GetGameInstance`)))
      (`ChronoGameInstance.PopInteractionCommand` _aschrono_game_instance (`InteractablePropBase.GetInteractionCommand` (`self.KeyToUse`))))))

(fn `DropKey`
  (bind _asbp_chrono_character (cast `/Game/Player/Blueprints/BP_ChronoCharacter` (`GameplayStatics.GetPlayerPawn` 0)))
  (`GrabbingAbility.DropObject` (`/Game/Player/Blueprints/BP_ChronoCharacter.GrabbingAbility` _asbp_chrono_character))
  (bind _aschrono_game_instance (cast `ChronoGameInstance` (`GameplayStatics.GetGameInstance`)))
  (`ChronoGameInstance.PopInteractionCommand` _aschrono_game_instance (`InteractablePropBase.GetInteractionCommand` (`self.KeyToUse`))))