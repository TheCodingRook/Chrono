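; Player character for a time-travel mechanic that spawns a past self replaying the player's recorded inputs.
; Traversing the level's TimePortal spawns that copy with its own controller at the starting transform, then a Tick-driven gate replays one timestamped entry per frame before wiping history.
; Tick tints the body by distance to the past self and kills both within the paradox threshold.
; Debug keys test alternative spawn and replay approaches.
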(event `Key|Two`
  (params (Key :type "Key Structure"))
  (bind _timetravel (`ChronoPlayerController.TimeTravel` (`self.GetMyChronoController`)))
  ;[1 0.2812 0] Replay historical movement and actions (create 2nd player version)
  (:`Pressed`
    (bind _pastself (`self.SpawSecondPlayer`))
    (`TimeTravelComponent.AllowRecording` _timetravel false)
    (set `self.PastSelfReference` _pastself)
    (bind _array_element (`/Game/GameFramework/CustomMacroLibrary.ForEachLoop(Custom-AllowsDelay)` (`TimeTravelComponent.GetTimestampedInputsArray` _timetravel) :!label _label)
      (:`LoopBody`
        (`KismetSystemLibrary.Delay` 1e-06)
        (`self.ReplayPastActions` _pastself _array_element)
        (goto _label :!via `Next Body`))
      (:`Completed`
        (`TimeTravelComponent.WipeHistory` _timetravel)))))

(event `BackInTime`
  (bind _iterator (`self.Iterator`))
  (bind _timetravel (`ChronoPlayerController.TimeTravel` (`self.GetMyChronoController`)))
  (bind _returnvalue (`TimeTravelComponent.GetTimestampedInputsArray` _timetravel))
  ;[0.03125 0 1] Replay historical actions - tick based approach
  (bind _spawnedcharacter (`self.SpawnPastSelf` :!label _label_2))
  (`TimeTravelComponent.AllowRecording` _timetravel false)
  (if (> (`KismetArrayLibrary.Array_Length` _returnvalue) 0)
    (goto _label_4 :!via `Open`)
    (else
      (goto _label_4 :!via `Close`))))

(event `Key|Q`
  (params (Key :type "Key Structure"))
  (bind _timetravel (`ChronoPlayerController.TimeTravel` (`self.GetMyChronoController`)))
  ;[0.07812 1 0] Replay historical movement and actions (spawn controller and possess new pawn version) - YAW/PITCH INPUTS NOT WORKING
  (:`Pressed`
    (bind _spawnedcharacter (`self.SpawnPastSelf`))
    (`TimeTravelComponent.AllowRecording` _timetravel false)
    (bind _array_element (`/Game/GameFramework/CustomMacroLibrary.ForEachLoop(Custom-AllowsDelay)` (`TimeTravelComponent.GetTimestampedInputsArray` _timetravel) :!label _label_3)
      (:`LoopBody`
        (`KismetSystemLibrary.Delay` 1e-05)
        (`self.ReplayPastActions` _spawnedcharacter _array_element)
        (goto _label_3 :!via `Next Body`))
      (:`Completed`
        (`TimeTravelComponent.WipeHistory` _timetravel)))))

(event `self.ReceiveBeginPlay`
  (`|ExecutionSequence`
    (:`then_0`
      ;[0.3828 1 0] Set starting transform for this character
      (set `self.StartingTransform` (`self.GetTransform` self)))
    (:`then_1`
      ;[0.3594 1 0] Find the TimePortals in the Level and bind delegates
      (bind _returnvalue (`GameplayStatics.GetActorOfClass` "/Game/TimePortals/Blueprints/BP_TimePortal.BP_TimePortal_C")) ; Find the TimePortal reference - PROBABLY SLOW
      (`/Engine/EditorBlueprintResources/StandardMacros.IsValid` _returnvalue
        (:`Is Valid`
          (bind _output_get (set `self.TimePortal` _returnvalue))
          (add `TimePortal.OnPortalTraversal` _output_get (delegate `BackInTime`)))))))

(event `Attempt Replay History`
  (bind _iterator (`self.Iterator`))
  (bind _timetravel (`ChronoPlayerController.TimeTravel` (`self.GetMyChronoController`)))
  (bind _returnvalue (`TimeTravelComponent.GetTimestampedInputsArray` _timetravel))
  ;[0.03125 0 1] Replay historical actions - tick based approach
  (`/Engine/EditorBlueprintResources/StandardMacros.Gate` true :!label _label_4
    (:`Exit`
      (`self.ReplayPastActions` (stale `BackInTime` _spawnedcharacter) (`|GetArrayItem` _returnvalue _iterator))
      (if (== _iterator (`KismetArrayLibrary.Array_LastIndex` _returnvalue))
        (`|ExecutionSequence`
          (:`then_0`
            (goto _label_4 :!via `Close`))
          (:`then_1`
            (`TimeTravelComponent.WipeHistory` _timetravel)))
        (else
          (`/Engine/EditorBlueprintResources/StandardMacros.IncrementInt` (`self.Iterator`)))))))

(event `Key|X`
  (params (Key :type "Key Structure"))
  ;[0.03125 0 1] Replay historical actions - tick based approach
  (:`Pressed`
    (goto _label_2)))

(event `Key|Z`
  (params (Key :type "Key Structure"))
  ;[1 0.2578 0] Replay historical movement and actions (for same character) - MOSTLY FOR DEBUGGING PURPOSES NOW
  (:`Pressed`
    (bind _aschrono_player_controller (cast `ChronoPlayerController` (`self.GetController`)))
    (bind _returnvalue (`ChronoPlayerController.GetTimeTravelComponent` _aschrono_player_controller))
    (`TimeTravelComponent.AllowRecording` _returnvalue false)
    (bind _array_element (`/Game/GameFramework/CustomMacroLibrary.ForEachLoop(Custom-AllowsDelay)` (`TimeTravelComponent.GetTimestampedInputsArray` _returnvalue) :!label _label_5)
      (:`LoopBody`
        (`KismetSystemLibrary.Delay` 1e-05)
        (`self.ReplayPastActions` _array_element)
        (goto _label_5 :!via `Next Body`)))))

(event `self.ReceiveTick`
  (params (DeltaSeconds :type "Float (single-precision)"))
  (`|ExecutionSequence`
    (:`then_0`
      (`self.Attempt Replay History`))
    (:`then_1`
      (`/Engine/EditorBlueprintResources/StandardMacros.IsValid` (`self.PastSelfReference`)
        (:`Is Valid`
          (bind _output_get (set `self.ProximityToPastSelf` (`KismetMathLibrary.VSize` (- (`self.K2_GetActorLocation` (`self.PastSelfReference`)) (`SceneComponent.K2_GetComponentLocation` (`self.Mesh`))))))
          (if (<= _output_get (`self.ParadoxThreshold`))
            ;[0 0.08594 1] Kill everyone!
            (`self.KillCharacter`)
            (`self.KillCharacter` (`self.PastSelfReference`))
            (else
              (bind _returnvalue (`PrimitiveComponent.CreateDynamicMaterialInstance` (`self.Mesh`) 0 null "None"))
              (`MaterialInstanceDynamic.SetVectorParameterValue` _returnvalue "BodyColor" (`KismetMathLibrary.LinearColorLerp` (struct :`R` 0.804166 :`B` 0.013236 :`A` 1.0) (struct :`R` 0.111958 :`G` 0.658333 :`A` 1.0) (/ (- (`self.ProximityToPastSelf`) (`self.ParadoxThreshold`)) (- (`self.AlertRadius`) (`self.ParadoxThreshold`))))))))))))

(fn `SpawnPastSelf`
  (returns (SpawnedCharacter :type "/Game/Player/Blueprints/BP_ChronoCharacter Object Reference"))
  (bind _startingtransform (`self.StartingTransform`))
  (bind _returnvalue (`|SpawnActorFromClass` "/Script/Chrono.ChronoPlayerController" _startingtransform "Undefined" "OverrideRootScale"))
  (bind _returnvalue_2 (`|SpawnActorFromClass` "BP_ChronoCharacter_C" _startingtransform "AdjustIfPossibleButAlwaysSpawn" "OverrideRootScale" null null))
  (`KismetArrayLibrary.Array_Add` (`Actor.Tags` _returnvalue_2) "Past self")
  (`Controller.Possess` _returnvalue _returnvalue_2)
  (set `self.PastSelfReference` _returnvalue_2)
  (`TimeTravelComponent.AllowRecording` (`ChronoPlayerController.GetTimeTravelComponent` _returnvalue) false)
  (return _returnvalue_2))

(fn `SpawSecondPlayer`
  (returns (PastSelf :type "/Game/Player/Blueprints/BP_ChronoCharacter Object Reference"))
  (bind _returnvalue (`GameplayStatics.CreatePlayer` -1))
  (bind _asbp_chrono_character (cast `/Game/Player/Blueprints/BP_ChronoCharacter` (`Controller.K2_GetPawn` _returnvalue))
    (:`then`
      (`KismetArrayLibrary.Array_Add` (`Actor.Tags` _asbp_chrono_character) "Past self") ; Designate as past self
      ;[0 0.25 1] Past self not allowed to record his actions
      (`TimeTravelComponent.AllowRecording` (`ChronoPlayerController.GetTimeTravelComponent` (`self.GetMyChronoController` _asbp_chrono_character)) false)
      (return _asbp_chrono_character))
    (:`CastFailed`
      (`KismetSystemLibrary.PrintString` "Cast to BP_ChronoCharacter failed in \"Spawn Second Player\" function"))))

(fn `UserConstructionScript`
  (bind _mesh (`self.Mesh`))
  (`|ExecutionSequence`
    (:`then_0`
      (bind _aschrono_player_controller (cast `ChronoPlayerController` (`self.GetController`)))
      (set `self.TimeTravel` (`ChronoPlayerController.GetTimeTravelComponent` _aschrono_player_controller)))
    (:`then_1`
      ;[0 1 0.1328] Change character's color
      (bind _returnvalue (`PrimitiveComponent.CreateDynamicMaterialInstance` _mesh 0 (`PrimitiveComponent.GetMaterial` _mesh 0) "None"))
      (set `self.TimeTravelMaterial` _returnvalue))))